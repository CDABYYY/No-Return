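; BP_Y_Ally is an ally character Blueprint that plays sections of a montage on its mesh through custom events.
; MyPlayMontage starts the section named by PlayName at a given play rate, first setting a same-named motion warping target from ToFloor's target location when Offset is true.
; PlayDead plays a named section of the same montage without warping.
; BeginPlay, Tick and overlap events are empty.
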(event `self.ReceiveBeginPlay`)

(event `self.MyPlayMontage`
  (params (PlayName :type Name) (ToFloor :type "Y_Floor Object Reference") (PlayRate :type "Float (single-precision)") (Offset :type Boolean))
  (if Offset
    (bind _returnvalue (`Y_Floor.TargetLocation` ToFloor))
    (`KismetSystemLibrary.PrintString` (`KismetStringLibrary.Conv_VectorToString` _returnvalue))
    (`MotionWarpingComponent.AddOrUpdateWarpTargetFromLocation` (`self.MotionWarping`) PlayName _returnvalue))
  (`|PlayMontage` (`self.Mesh`) (`self.Montage to Play`) PlayRate 0.0 PlayName))

(event `self.PlayDead`
  (params (MontageName :type Name))
  (`|PlayMontage` (`self.Mesh`) (`self.Montage to Play`) 1.0 0.0 MontageName))

(fn `UserConstructionScript`)