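; BP_Y_PlayerController is a player controller that creates and shows the game's map, event, room settlement and HUD widgets.
; Map events create or rebuild TestMapWidget, have its inner map widget run GetMap, and slide it open or closed by playing PullMap forward or in reverse.
; The event panel animates in the same way and is removed after a delay on close.
; EndRoom and LoadHUD create and initialise their widgets.
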(event `self.ReceiveBeginPlay`)

(event `self.ShowMap`
  (bind _testmapwidget (`self.TestMapWidget`))
  (`UserWidget.PlayAnimation` _testmapwidget (`/Game/BluePrint/TestMapWidget.PullMap` _testmapwidget) 0.0 1 "Forward" 1.0 false))

(event `self.CloseMap`
  (bind _testmapwidget (`self.TestMapWidget`))
  (`UserWidget.PlayAnimation` _testmapwidget (`/Game/BluePrint/TestMapWidget.PullMap` _testmapwidget) 0.0 1 "Reverse" 1.0 false))

(event `self.UpdateMap`
  (`/Engine/EditorBlueprintResources/StandardMacros.IsValid` (`self.TestMapWidget`)
    (:`Is Valid`
      (`Widget.RemoveFromParent` (`self.TestMapWidget`)))
    (:`Is Not Valid`
      _))
  (bind _returnvalue (`|CreateWidget` "/Game/BluePrint/TestMapWidget.TestMapWidget_C" self))
  (set `self.TestMapWidget` _returnvalue)
  (bind _bp_y_mapwidget (`/Game/BluePrint/TestMapWidget.BP_Y_MapWidget` _returnvalue))
  (set `self.MapWidget` _bp_y_mapwidget)
  (`Y_MapWidget.GetMap` _bp_y_mapwidget)
  (`UserWidget.AddToViewport` _returnvalue 0))

(event `self.ShowEvent`
  (bind _returnvalue (`|CreateWidget` "/Game/BluePrint/BP_Y_EventWidget.BP_Y_EventWidget_C" self))
  (set `self.EventWidget` _returnvalue)
  (set `self.BPEvent` _returnvalue)
  (`UserWidget.AddToViewport` _returnvalue 0)
  (`UserWidget.PlayAnimation` _returnvalue (`/Game/BluePrint/BP_Y_EventWidget.PullEventAnimation` _returnvalue) 0.0 1 "Forward" 1.0 false))

(event `self.CloseEvent`
  (bind _bpevent (`self.BPEvent`))
  (`UserWidget.PlayAnimation` _bpevent (`/Game/BluePrint/BP_Y_EventWidget.PullEventAnimation` _bpevent) 0.0 1 "Reverse" 1.0 false)
  (`KismetSystemLibrary.Delay` 2.0)
  (`Widget.RemoveFromParent` _bpevent))

(event `self.LoadMap`
  (bind _returnvalue (`|CreateWidget` "/Game/BluePrint/TestMapWidget.TestMapWidget_C" self))
  (set `self.TestMapWidget` _returnvalue)
  (bind _bp_y_mapwidget (`/Game/BluePrint/TestMapWidget.BP_Y_MapWidget` _returnvalue))
  (set `self.MapWidget` _bp_y_mapwidget)
  (`Y_MapWidget.GetMap` _bp_y_mapwidget)
  (`UserWidget.AddToViewport` _returnvalue 0))

(event `self.EndRoom`
  (bind _returnvalue (`|CreateWidget` "/Game/BluePrint/BP_Settle.BP_Settle_C" self))
  (`Y_Settle.Init` _returnvalue)
  (`UserWidget.AddToViewport` _returnvalue 0))

(event `self.LoadHUD`
  (bind _returnvalue (`|CreateWidget` "/Game/BluePrint/BP_Y_HUD.BP_Y_HUD_C" self))
  (bind _output_get (set `self.PCHUD` _returnvalue))
  (`Y_HUD.HUDInit` _output_get)
  (`UserWidget.AddToViewport` _returnvalue 0))

(fn `UserConstructionScript`)