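; Player camera pawn that shows a begin widget on BeginPlay and serves as an input hub with debug-style hotkeys.
; Left mouse press and release, plus an experiment key, forward to functions defined outside this graph.
; Other keys open a debug widget, play the HUD's pass-notice animation, or end the room through the game instance.
; Unconnected leftover nodes hold event and map widget toggles, card/floor click tracing and hover-outline highlighting.
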(event `self.ReceiveBeginPlay`
  (bind _returnvalue (`|CreateWidget` "/Game/UIBlueprints/BeginWidget.BeginWidget_C"))
  (`UserWidget.AddToViewport` _returnvalue 0))

(event `Key|M`
  (params (Key :type "Key Structure"))
  (:`Pressed`
    (bind _returnvalue (`|CreateWidget` "/Game/UIBlueprints/DebugWidget.DebugWidget_C"))
    (`UserWidget.AddToViewport` _returnvalue 0)))

(event `Key|E`
  (params (Key :type "Key Structure"))
  (:`Pressed`
    (`self.TryExperimentFunction`)))

(event `Key|LeftMouseButton`
  (params (Key :type "Key Structure"))
  (:`Pressed`
    (`self.MouseLeftPress`))
  (:`Released`
    (`self.MouseLeftRelease`)))

(event `Key|F`
  (params (Key :type "Key Structure")))

(event `Key|T`
  (params (Key :type "Key Structure"))
  (:`Pressed`
    (bind _asy_player_controller (cast `Y_PlayerController` (`self.GetController`)))
    (bind _myy_hud (`Y_PlayerController.MyY_HUD` _asy_player_controller))
    (bind _asbp_y_hud (cast `/Game/BluePrint/BP_Y_HUD` _myy_hud))
    (`UserWidget.PlayAnimation` _myy_hud (`/Game/BluePrint/BP_Y_HUD.PassNotice` _asbp_y_hud) 0.0 1 "Forward" 1.0 false)))

(event `Key|Y`
  (params (Key :type "Key Structure"))
  (:`Pressed`
    (bind _asy_game_instance (cast `Y_GameInstance` (`GameplayStatics.GetGameInstance`)))
    (`Y_GameInstance.EndRoom` _asy_game_instance)))

(event `Key|G`
  (params (Key :type "Key Structure")))

(fn `UserConstructionScript`)