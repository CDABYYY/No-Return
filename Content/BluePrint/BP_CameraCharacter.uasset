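; Camera character Blueprint that lets the player click a static mesh in the world to highlight it as the current selection.
; On left mouse press, it deprojects the cursor and runs a long Visibility line trace.
; A hit static mesh component gets a blue overlay material and custom depth, after the previously stored component is cleared.
; Clicks that hit no static mesh leave the current highlight in place.
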(event `Key|LeftMouseButton`
  (params (Key :type "Key Structure"))
  (bind (_worldlocation _worlddirection) (`PlayerController.DeprojectMousePositionToWorld` (`GameplayStatics.GetPlayerController` 0)))
  (:`Pressed`
    (bind _outhit (`KismetSystemLibrary.LineTraceSingle` _worldlocation (+ _worldlocation (* _worlddirection 100000)) "TraceTypeQuery1"))
    (bind `_as静态网格体组件` (cast `StaticMeshComponent` (`.HitComponent` (`GameplayStatics.BreakHitResult` _outhit))))
    (bind `_as静态网格体组件_2` (`self.As静态网格体组件`)
      (:`then`
        (`MeshComponent.SetOverlayMaterial` `_as静态网格体组件_2` null)
        (`PrimitiveComponent.SetRenderCustomDepth` `_as静态网格体组件_2` false))
      (:`else`
        _))
    (`PrimitiveComponent.SetRenderCustomDepth` `_as静态网格体组件` true)
    (`MeshComponent.SetOverlayMaterial` `_as静态网格体组件` "/Game/Resource/Material/BlueMaterialInstance.BlueMaterialInstance")
    (set `self.As静态网格体组件` `_as静态网格体组件`)))

(fn `UserConstructionScript`)