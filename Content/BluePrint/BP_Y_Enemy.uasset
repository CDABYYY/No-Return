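; BP_Y_Enemy is an enemy that exposes events for montage animation, death and visual effects.
; MyPlayMontage plays a named montage section, optionally updating a same-named motion warp target from a floor location, then clears the first Niagara slot and prints debug positions on completion.
; PlayDead destroys the actor on a "Die" notify.
; PlayNiagara looks up GameInstance maps by name to set an overlay material or one of three Niagara slots.
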(event `self.MyPlayMontage`
  (params (PlayName :type Name) (ToFloor :type "Y_Floor Object Reference") (PlayRate :type "Float (single-precision)") (Offset :type Boolean))
  (if Offset
    (bind _returnvalue (`Y_Floor.TargetLocation` ToFloor))
    (set `self.GetDistance` _returnvalue)
    (`MotionWarpingComponent.AddOrUpdateWarpTarget` (`self.MotionWarping`) (make `MotionWarpingTarget` PlayName _returnvalue (`self.K2_GetActorRotation`))))
  (`|PlayMontage` (`self.Mesh`) (`self.Montage to Play`) PlayRate 0.0 PlayName
    (:`OnCompleted`
      (`NiagaraComponent.SetAsset` (`self.Niagara1`) null true)
      (`KismetSystemLibrary.PrintString` (`KismetStringLibrary.Conv_VectorToString` (`self.GetDistance`)))
      (`KismetSystemLibrary.PrintString` (`KismetStringLibrary.Conv_VectorToString` (`self.K2_GetActorLocation`))))))

(event `self.PlayDead`
  (params (MontageName :type Name))
  (bind _notifyname (`|PlayMontage` (`self.Mesh`) (`self.Montage to Play`) 1.0 0.0 MontageName)
    (:`OnNotifyBegin`
      (if (== _notifyname "Die")
        (`self.K2_DestroyActor`)))))

(event `self.PlayNiagara`
  (params (Type :type Integer) (PlayName :type Name))
  (bind _asbp_y_game_instance (cast `/Game/BluePrint/BP_Y_GameInstance` (`GameplayStatics.GetGameInstance`)))
  (switch `int` Type
    (:`0`
      (`MeshComponent.SetOverlayMaterial` (`self.Mesh`) (`BlueprintMapLibrary.Map_Find` (`/Game/BluePrint/BP_Y_GameInstance.BodyNiagara` _asbp_y_game_instance) PlayName))
      (set `self.CurrentOverlap` PlayName))
    (:`1`
      (bind _value (`BlueprintMapLibrary.Map_Find` (`/Game/BluePrint/BP_Y_GameInstance.BoneNiagara` _asbp_y_game_instance) PlayName))
      (`NiagaraComponent.SetAsset` (`self.Niagara1`) _value true)
      (set `self.CurrentNiagara` PlayName))
    (:`2`
      (`NiagaraComponent.SetAsset` (`self.Niagara2`) _value true))
    (:`3`
      (`NiagaraComponent.SetAsset` (`self.Niagara3`) _value true))))

(fn `UserConstructionScript`)